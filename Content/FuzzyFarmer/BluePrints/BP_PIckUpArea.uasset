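; BP_PIckUpArea is a pickup zone that may spawn a BP_Item at one of three spawn points on BeginPlay.
; SpawnPoints loops over every BP_PIckUpArea, overwriting three stored locations each pass, so only the last area's points remain.
; SpawnCoins then rolls a random integer, spawning one narrowed item at a stored location on three of seven outcomes, otherwise nothing.
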(event `self.ReceiveBeginPlay`
  (`self.SpawnPoints`)
  (`self.SpawnCoins`))

(fn `SpawnCoins`
  (switch `int` (`KismetMathLibrary.RandomIntegerInRange` 0 6)
    (:`0`
      (`|SpawnActorFromClass` "/Game/FuzzyFarmer/BluePrints/BP_Item.BP_Item_C" (`KismetMathLibrary.MakeTransform` (`self.SP1_WorldLocation`) (struct) (0.25 1.0 1.0)) "Undefined" "OverrideRootScale" null null))
    (:`3`
      (`|SpawnActorFromClass` "/Game/FuzzyFarmer/BluePrints/BP_Item.BP_Item_C" (`KismetMathLibrary.MakeTransform` (`self.SP2_WorldLocation`) (struct) (0.25 1.0 1.0)) "Undefined" "OverrideRootScale" null null))
    (:`6`
      (`|SpawnActorFromClass` "/Game/FuzzyFarmer/BluePrints/BP_Item.BP_Item_C" (`KismetMathLibrary.MakeTransform` (`self.SP3_WorldLocation`) (struct) (0.25 1.0 1.0)) "Undefined" "OverrideRootScale" null null))))

(fn `SpawnPoints`
  (bind _outactors (`GameplayStatics.GetAllActorsOfClass` "BP_PIckUpArea_C"))
  (for _array_element _outactors
    (set `self.SP1_WorldLocation` (`SceneComponent.K2_GetComponentLocation` (`/Game/FuzzyFarmer/BluePrints/BP_PIckUpArea.SpawnPoint1` _array_element)))
    (set `self.SP2_WorldLocation` (`SceneComponent.K2_GetComponentLocation` (`/Game/FuzzyFarmer/BluePrints/BP_PIckUpArea.SpawnPoint2` _array_element)))
    (set `self.SP3_WorldLocation` (`SceneComponent.K2_GetComponentLocation` (`/Game/FuzzyFarmer/BluePrints/BP_PIckUpArea.SpawnPoint3` _array_element)))))

(fn `UserConstructionScript`)