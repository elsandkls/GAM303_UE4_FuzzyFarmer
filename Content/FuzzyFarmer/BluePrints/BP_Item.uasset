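; BP_Item is a time coin pickup that adds its TimeValue to the ThirdPersonCharacter's Minutes.
; BeginPlay caches the player character, and overlapping the Trigger collects the coin immediately, hiding it, updating the time and destroying it after a short delay.
; Separate events raise or lower the character's TotalTimeCoins, but nothing in this graph calls them.
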(event `self.ReceiveBeginPlay`
  (bind _asthird_person_character (cast `/Game/ThirdPersonBP/Blueprints/ThirdPersonCharacter` (`GameplayStatics.GetPlayerCharacter` 0)))
  (set `self.CharacterReference` _asthird_person_character))

(event `self.Trigger.OnComponentBeginOverlap`
  (params (OverlappedComponent :type "PrimitiveComponent Object Reference") (OtherActor :type "Actor Object Reference") (OtherComp :type "PrimitiveComponent Object Reference") (OtherBodyIndex :type Integer) (bFromSweep :type Boolean) (SweepResult :type "HitResult Structure (by ref)"))
  ;[1 1 1] Overlap Trigger for pickup text
  (cast `/Game/ThirdPersonBP/Blueprints/ThirdPersonCharacter` OtherActor)
  (set `self.IsInRange` true)
  (`self.OnPickUp`))

(event `self.Trigger.OnComponentEndOverlap`
  (params (OverlappedComponent :type "PrimitiveComponent Object Reference") (OtherActor :type "Actor Object Reference") (OtherComp :type "PrimitiveComponent Object Reference") (OtherBodyIndex :type Integer))
  ;[1 1 1] Overlap Trigger for pickup text
  (cast `/Game/ThirdPersonBP/Blueprints/ThirdPersonCharacter` OtherActor)
  (set `self.IsInRange` false))

(event `UpdateTime`
  (bind _characterreference (`self.CharacterReference`))
  ;[1 1 1] Update Time Value When Coin is Picked Up
  (set `/Game/ThirdPersonBP/Blueprints/ThirdPersonCharacter.Minutes` (+ (`self.TimeValue`) (`/Game/ThirdPersonBP/Blueprints/ThirdPersonCharacter.Minutes` _characterreference)) _characterreference))

(event `OnPickUp`
  ;[1 1 1] Delete actor from level after being picked up.
  (set `self.IsInRange` false)
  (`self.SetActorHiddenInGame` true)
  (`self.UpdateTime`)
  (`KismetSystemLibrary.Delay` 2.0)
  (`self.K2_DestroyActor` self))

(event `IncreaseCoinCount`
  (bind _characterreference (`self.CharacterReference`))
  ;[1 1 1] Coin Count Adjustments
  (set `/Game/ThirdPersonBP/Blueprints/ThirdPersonCharacter.TotalTimeCoins` (+ (`/Game/ThirdPersonBP/Blueprints/ThirdPersonCharacter.TotalTimeCoins` _characterreference) 1) _characterreference))

(event `DecreaseCoinCount`
  (bind _characterreference (`self.CharacterReference`))
  ;[1 1 1] Coin Count Adjustments
  (set `/Game/ThirdPersonBP/Blueprints/ThirdPersonCharacter.TotalTimeCoins` (- (`/Game/ThirdPersonBP/Blueprints/ThirdPersonCharacter.TotalTimeCoins` _characterreference) 1) _characterreference))

(fn `UserConstructionScript`)